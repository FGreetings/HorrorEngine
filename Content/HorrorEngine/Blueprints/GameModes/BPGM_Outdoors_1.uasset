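; Outdoors game mode for HorrorEngine, holding logic to restore the player's saved level and position.
; CharacterSpawn loads the gameplay save from its slot, or creates a new save object if none exists.
; SaveGameCheck streams in the saved level, then teleports the player pawn to the saved transform if that level is loaded.
; BeginPlay is empty and the only CharacterSpawn call is disconnected, so nothing here triggers the restore.
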(event `self.ReceiveBeginPlay`)

(event `CharacterSpawn`
  (bind _returnvalue (`GameplayStatics.DoesSaveGameExist` (`self.SlotName`)))
  (if _returnvalue
    (bind _returnvalue_2 (`GameplayStatics.LoadGameFromSlot` (`self.SlotName`)))
    (bind _output_get (set `self.SaveSubClass` _returnvalue_2))
    (bind _asbpsg_gameplay_save_game (cast `/Game/HorrorEngine/Blueprints/SaveGames/BPSG_GameplaysaveGame` _output_get))
    (`self.SaveGameCheck` _asbpsg_gameplay_save_game)
    (else
      (bind _returnvalue_3 (`GameplayStatics.CreateSaveGameObject` "/Game/HorrorEngine/Blueprints/SaveGames/BPSG_GameplaysaveGame.BPSG_GameplaySaveGame_C"))
      (bind _output_get_2 (set `self.SaveSubClass` _returnvalue_3))
      (bind _asbpsg_gameplay_save_game_2 (cast `/Game/HorrorEngine/Blueprints/SaveGames/BPSG_GameplaysaveGame` _output_get_2))
      (`self.SaveGameCheck` _asbpsg_gameplay_save_game_2))))

(event `SaveGameCheck`
  (params (GameplaySaveGame :type "/Game/HorrorEngine/Blueprints/SaveGames/BPSG_GameplaysaveGame Object Reference"))
  (bind _streamlevelname (`/Game/HorrorEngine/Blueprints/SaveGames/BPSG_GameplaysaveGame.StreamLevelName` GameplaySaveGame))
  (`GameplayStatics.LoadStreamLevel` _streamlevelname true)
  (if (`LevelStreaming.IsLevelLoaded` (`GameplayStatics.GetStreamingLevel` _streamlevelname))
    (bind _returnvalue (`self.K2_TeleportTo` (`GameplayStatics.GetPlayerPawn` 0) (`/Game/HorrorEngine/Blueprints/SaveGames/BPSG_GameplaysaveGame.PlayerLocation` GameplaySaveGame) (`/Game/HorrorEngine/Blueprints/SaveGames/BPSG_GameplaysaveGame.PlayerRotation` GameplaySaveGame)))
    (`KismetSystemLibrary.PrintString` (`KismetStringLibrary.Conv_BoolToString` _returnvalue))))

(fn `UserConstructionScript`)