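; Checkpoint actor that records a player respawn transform and writes it to the gameplay save slot.
; When a HorrorEngineCharacter overlaps its box, it stores the world location and rotation of an arrow component.
; A separate SaveGameCheck event, not called within this graph, loads or creates BPSG_GameplaySaveGame.
; SaveToGameSlot then writes the stored transform and checkpoint streaming level name into that object and saves it.
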(event `self.Box.OnComponentBeginOverlap`
  (params (OverlappedComponent :type "PrimitiveComponent Object Reference") (OtherActor :type "Actor Object Reference") (OtherComp :type "PrimitiveComponent Object Reference") (OtherBodyIndex :type Integer) (bFromSweep :type Boolean) (SweepResult :type "HitResult Structure (by ref)"))
  (bind _arrowforloc_rot (`self.ArrowForLoc&Rot`))
  (cast `/Game/HorrorEngine/Blueprints/Core/HorrorEngineCharacter` OtherActor)
  (set `self.CheckPointLocation` (`SceneComponent.K2_GetComponentLocation` _arrowforloc_rot))
  (set `self.CheckPointRotation` (`SceneComponent.K2_GetComponentRotation` _arrowforloc_rot)))

(event `SaveGameCheck`
  (bind _returnvalue (`GameplayStatics.DoesSaveGameExist` (`self.SlotName`)))
  (if _returnvalue
    (bind _returnvalue_2 (`GameplayStatics.LoadGameFromSlot` (`self.SlotName`)))
    (bind _output_get (set `self.SaveSubClass` _returnvalue_2))
    (bind _asbpsg_gameplay_save_game (cast `/Game/HorrorEngine/Blueprints/SaveGames/BPSG_GameplaysaveGame` _output_get))
    (`self.SaveToGameSlot` _asbpsg_gameplay_save_game)
    (else
      (bind _returnvalue_3 (`GameplayStatics.CreateSaveGameObject` "/Game/HorrorEngine/Blueprints/SaveGames/BPSG_GameplaysaveGame.BPSG_GameplaySaveGame_C"))
      (bind _output_get_2 (set `self.SaveSubClass` _returnvalue_3))
      (bind _asbpsg_gameplay_save_game_2 (cast `/Game/HorrorEngine/Blueprints/SaveGames/BPSG_GameplaysaveGame` _output_get_2))
      (`self.SaveToGameSlot` _asbpsg_gameplay_save_game_2))))

(event `SaveToGameSlot`
  (params (GameplaySaveGame :type "/Game/HorrorEngine/Blueprints/SaveGames/BPSG_GameplaysaveGame Object Reference"))
  (set `/Game/HorrorEngine/Blueprints/SaveGames/BPSG_GameplaysaveGame.PlayerLocation` (`self.CheckPointLocation`) GameplaySaveGame)
  (set `/Game/HorrorEngine/Blueprints/SaveGames/BPSG_GameplaysaveGame.PlayerRotation` (`self.CheckPointRotation`) GameplaySaveGame)
  (set `/Game/HorrorEngine/Blueprints/SaveGames/BPSG_GameplaysaveGame.StreamLevelName` (`self.CheckPointLevelName`) GameplaySaveGame)
  (`GameplayStatics.SaveGameToSlot` (`self.SaveSubClass`) (`self.SlotName`)))

(fn `UserConstructionScript`
  (`parent.UserConstructionScript`))